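; Wind controller Blueprint that drives a global, gradually shifting wind direction for materials.
; BeginPlay loops through a fixed set of horizontal target directions, switching after a timed delay.
; Each Tick writes the current direction into the MP_Global parameter collection's "Wind Direction" vector, then lerps it a small step toward the target, so easing is frame-rate dependent.
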(event EventBeginPlay
  (Variables|Default|SetTargetWIndDirection "0.000000,-200.000000,0.000000" :!label _label)
  (Utilities|FlowControl|Delay 2e+01)
  (Variables|Default|SetTargetWIndDirection "200.000000,-200.000000, 0")
  (Utilities|FlowControl|Delay 2e+01)
  (Variables|Default|SetTargetWIndDirection "200.000000,0.000000, 0")
  (Utilities|FlowControl|Delay 2e+01)
  (Variables|Default|SetTargetWIndDirection "200.000000,200.000000, 0")
  (Utilities|FlowControl|Delay 2e+01)
  (Variables|Default|SetTargetWIndDirection "0.000000,200.000000, 0")
  (Utilities|FlowControl|Delay 2e+01)
  (goto _label))

(event Collision|EventActorBeginOverlap
  (params (OtherActor :type Actor%20Object%20Reference)))

(event EventTick
  (params (DeltaSeconds :type Float%20%28single-precision%29))
  (|UpdateWIndDirection))

(fn ConstructionScript)