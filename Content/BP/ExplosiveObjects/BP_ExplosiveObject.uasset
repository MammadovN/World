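; BP_ExplosiveObject is a destructible object that explodes when hit by a Fire arrow or another explosion.
; Explode runs once, spawning effects, sound and a burn decal, applying radius damage to its destructible mesh.
; A sphere trace sends OnFireHit to nearby destructibles and pawns; receiving explosives detonate after a random delay, creating chain reactions.
; Two timelines grow then shrink a global material parameter collection's explosion radius around the blast origin.
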(event Custom|Explode
  (bind _returnvalue (Transformation|GetActorLocation))
  (bind _returnvalue_2 (Transformation|GetActorLocation))
  (Utilities|FlowControl|DoOnce false
    (:Completed
      (Effects|SpawnEmitteratLocation "/Game/StarterContentMin/Particles/P_Explosion.P_Explosion" _returnvalue_2 "0, 0, 0" "3.000000,3.000000,3.000000")
      (Class|DestructibleComponent|ApplyRadiusDamage (Variables|Default|GetDestructible%20Mesh) 1.0 _returnvalue_2 2e+02 1e+03 true)
      (Audio|PlaySoundatLocation "/Game/StarterContentMin/Audio/Explosion_Cue.Explosion_Cue" _returnvalue_2 "0, 0, 0" 1.0 1.0 0.0 0 0 0)
      (|ExplodeSurroundingObjects
        (:Completed
          (Rendering|Decal|SpawnDecalatLocation "/Game/Materials/M_Burning.M_Burning" "128.000000,256.000000,256.000000" _returnvalue "-90.000000,0.000000,0.000000" 0.0)
          (Rendering|Material|SetVectorParameterValue "/Game/Materials/MP_Global.MP_Global" "ExplosionOrigin" (Math|Conversions|ToLinearColor(Vector) _returnvalue) :!class /Script/Engine.KismetMaterialLibrary)
          (bind _time (Timeline|Timeline_Explosion_out Play)
            (:Update
              (Rendering|Material|SetScalarParameterValue "/Game/Materials/MP_Global.MP_Global" "ExplosionRadius" (* _time 1e+03) :!class /Script/Engine.KismetMaterialLibrary))
            (:Finished
              (bind _time_2 (Timeline|Timeline_0 Play)
                (:Update
                  (Rendering|Material|SetScalarParameterValue "/Game/Materials/MP_Global.MP_Global" "ExplosionRadius" (* (Math|Float|Clamp(Float) (/ (- 1e+01 _time_2) 1e+01) 0.2) 1e+03) :!class /Script/Engine.KismetMaterialLibrary))))))))))

(event EventBeginPlay)

(event Collision|EventActorBeginOverlap
  (params (OtherActor :type Actor%20Object%20Reference)))

(event EventTick
  (params (DeltaSeconds :type Float%20%28single-precision%29)))

(event EventOnFireHit
  (params (source%20actor :type Actor%20Object%20Reference))
  (Utilities|FlowControl|Delay (Math|Random|RandomFloatinRange 0.5 2.0))
  (CallFunction|Explode))

(fn ConstructionScript)

(event EventOnArrowHit
  (params (hit%20location :type Vector :default "0, 0, 0") (source%20actor :type Actor%20Object%20Reference) (arrow :type Actor%20Object%20Reference))
  (bind _type (Class|BPIMagicalObject|GetMagicType(Message) arrow))
  (switch Utilities|FlowControl|Switch|SwitchonMagicType _type
    (:NewEnumerator1
      (CallFunction|Explode))))