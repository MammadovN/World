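; BP_Road is a spline-based road that populates itself with pedestrians and supplies path points along its length.
; On BeginPlay it spawns random ActorType classes at randomized spacing along the spline, stores them and passes itself to each via SetRoadMessage.
; GetNextPoint returns the world point at a given distance or flags the end.
; GetClosestPoint samples at fixed intervals; its MinDistance output is actually distance along the spline.
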(event EventBeginPlay
  (CallFunction|SpawnPedestrians))

(event Collision|EventActorBeginOverlap
  (params (OtherActor :type Actor%20Object%20Reference)))

(event EventTick
  (params (DeltaSeconds :type Float%20%28single-precision%29)))

(fn ConstructionScript)

(fn GetNextPoint
  (params (targetDistance :type Float%20%28single-precision%29))
  (bind _spline (Variables|Default|GetSpline))
  (if (and (> targetDistance 0.0) (< targetDistance (Spline|GetSplineLength _spline)))
    (return false (Spline|GetLocationatDistanceAlongSpline _spline targetDistance "World"))
    (else
      (return true "0, 0, 0"))))

(fn GetClosestPoint
  (params (location :type Vector))
  (bind _spline (Variables|Default|GetSpline))
  (if (> (Spline|GetSplineLength _spline) (LocalVariables|Getdistance)) :!label _label
    (if (> (LocalVariables|GetminDistance) (Math|Vector|Distance(Vector) location (Spline|GetLocationatDistanceAlongSpline _spline (LocalVariables|Getdistance) "World")))
      (LocalVariables|SetminDistance (Math|Vector|Distance(Vector) location (Spline|GetLocationatDistanceAlongSpline _spline (LocalVariables|Getdistance) "World")))
      (LocalVariables|Setclosest%20point (Spline|GetLocationatDistanceAlongSpline _spline (LocalVariables|Getdistance) "World"))
      (LocalVariables|SetclosestSplineLength (LocalVariables|Getdistance)))
    (LocalVariables|Setdistance (+ (LocalVariables|Getdistance) 5e+02))
    (goto _label)
    (else
      (return (LocalVariables|Getclosest%20point) (LocalVariables|GetclosestSplineLength)))))

(fn SpawnPedestrians
  (bind _spline (Variables|Default|GetSpline))
  (bind _actor_distance (Variables|Default|Getactor%20distance))
  (if (> (Spline|GetSplineLength _spline) (LocalVariables|Getdistance)) :!label _label
    (bind _returnvalue (Game|SpawnActorfromClass (CallFunction|GetActorType) (Math|Transform|MakeTransform (+ (Spline|GetLocationatDistanceAlongSpline _spline (LocalVariables|Getdistance) "World") "0, 0,100.000000") "0, 0, 0" "1,1,1") "Undefined" 0 0))
    (Utilities|IsValid _returnvalue
      (:Is%20Valid
        (Utilities|Array|Add (Variables|Default|Getspawned%20actors) _returnvalue)
        (Class|BPIPedestrians|SetRoad(Message) _returnvalue self))
      (:Is%20Not%20Valid
        _))
    (LocalVariables|Setdistance (+ (LocalVariables|Getdistance) (+ _actor_distance (Math|Random|RandomFloatinRange 0.0 (/ _actor_distance 2.0)))))
    (goto _label)))

(fn GetActorType
  (bind _actor_type (Variables|Default|Getactor%20type))
  (return (Utilities|Array|Get(acopy) _actor_type (Math|Random|RandomInteger (Utilities|Array|Length _actor_type)))))