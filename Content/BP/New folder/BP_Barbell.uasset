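; BP_Barbell is an interactable barbell that makes a character perform a clean and jerk.
; On interaction it flips 180 degrees if the second stand point is nearer, locks movement, disables barbell collision and eases the character into place.
; A montage's "Grab" notify attaches the bar to the right hand; other notifies end the interaction.
; Release returns the bar and restores movement, but the collision re-enable is unwired.
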(event Custom|ReleaseBarbell
  (bind _barbell (Variables|Default|GetBarbell))
  (bind _originaltransform (Variables|Default|GetOriginalTransform))
  (Transformation|AttachComponentToComponent _barbell (Variables|Default|GetDefaultSceneRoot) "None" "KeepWorld" "KeepWorld" "KeepWorld" true)
  (Components|MoveComponentTo _barbell (.location _originaltransform) (.rotation _originaltransform) false false 0.2 false)
  (Class|BPICharacter|ToggleMovement(Message) (Variables|Default|GetCharacter) true))

(event EventBeginPlay
  (|CallParentFunction)
  (Variables|Default|SetOriginalTransform (Transformation|GetRelativeTransform (Variables|Default|GetBarbell))))

(event Collision|EventActorBeginOverlap
  (params (OtherActor :type Actor%20Object%20Reference))
  (|CallParentFunction OtherActor) ; This node is disabled and will not be called.\nDrag off pins to build functionality.
)

(event EventTick
  (params (DeltaSeconds :type Float%20%28single-precision%29))
  (|CallParentFunction DeltaSeconds) ; This node is disabled and will not be called.\nDrag off pins to build functionality.
)

(event EventStartInteraction
  (params (InteractingCharacter :type Actor%20Object%20Reference))
  (bind _characterlocation1 (Variables|Default|GetCharacterLocation1))
  (bind _barbell (Variables|Default|GetBarbell))
  (bind _returnvalue (Transformation|GetWorldLocation _characterlocation1))
  (|CallParentFunction InteractingCharacter)
  (Variables|Default|SetActionCompleted false)
  (bind _ascharacter (Utilities|Casting|CastToCharacter (Variables|Default|GetInteractingActor)))
  (bind _output_get (Variables|Default|SetCharacter _ascharacter))
  (CallFunction|CheckSide)
  (Class|BPICharacter|ToggleMovement(Message) _output_get false)
  (Collision|SetCollisionEnabled (Variables|Default|GetBarbell) "NoCollision")
  (Utilities|FlowControl|Sequence
    (:then_0
      (Components|MoveComponentTo (Variables|/Script/Engine.Actor|GetRootComponent (Variables|Default|GetInteractingActor)) (Math|Vector|MakeVector (.x _returnvalue) (.y _returnvalue) (+ (.z _returnvalue) (Variables|/Script/Engine.CapsuleComponent|GetCapsuleHalfHeight (Variables|/Script/Engine.Character|GetCapsuleComponent (Variables|Default|GetCharacter))))) (Transformation|GetWorldRotation _characterlocation1) true true 0.5 false))
    (:then_1
      (bind _notifyname (Animation|Montage|PlayMontage (Variables|/Script/Engine.Character|GetMesh (Variables|Default|GetCharacter)) "/Game/Characters/Mannequins/Animations/Manny/AI_Actions/Clean_And_Jerk_Montage.Clean_And_Jerk_Montage")
        (:OnNotifyBegin
          (if (== _notifyname "Grab")
            (Transformation|AttachComponentToComponent _barbell (Variables|/Script/Engine.Character|GetMesh (Variables|Default|GetCharacter)) "hand_rSocket" "KeepWorld" "KeepWorld" "KeepWorld" true)
            (Components|MoveComponentTo _barbell "0, 0, 0" "0, 0, 0" true true 0.2 false)
            (else
              (Variables|Default|SetActionCompleted true)
              (CallFunction|EndInteraction))))))))

(fn ConstructionScript
  (|CallParentFunction))

(fn CheckSide
  (bind _returnvalue (Transformation|GetActorRotation))
  (bind _interactingactor (Variables|Default|GetInteractingActor))
  (bind _returnvalue_2 (Transformation|GetActorLocation _interactingactor))
  (if (> (Math|Vector|Distance(Vector) _returnvalue_2 (Transformation|GetWorldLocation (Variables|Default|GetCharacterLocation1))) (Math|Vector|Distance(Vector) _returnvalue_2 (Transformation|GetWorldLocation (Variables|Default|GetCharacterLocation2))))
    (Transformation|SetActorRotation (Math|Rotator|MakeRotator (.roll _returnvalue) (.pitch _returnvalue) (+ (.yaw _returnvalue) 1.8e+02)))))

(fn EndInteraction
  (if (Variables|Default|GetActionCompleted)
    (|CallParentFunction)
    (CallFunction|ReleaseBarbell)
    (return true)
    (else
      (return false))))