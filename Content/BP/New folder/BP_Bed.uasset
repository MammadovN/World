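; BP_Bed is an interactable bed that lets a character lie down on it and get back up.
; Starting interaction turns off the character's movement message, plays a lie-down montage and eases the capsule onto the bed's location and yaw.
; Ending interaction calls ReleaseChair, which plays a stand-up montage, then on blend out moves the character to the exit point and restores the movement message.
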(event Custom|ReleaseChair
  (bind _character (Variables|Default|GetCharacter))
  (bind _character_2 (Variables|Default|GetCharacter)
    (:then
      (Animation|Montage|PlayMontage (Variables|/Script/Engine.Character|GetMesh _character_2) "/Game/Characters/Mannequins/Animations/Manny/AI_Actions/Stand_Up.Stand_Up"
        (:OnBlendOut
          (Components|MoveComponentTo (Variables|/Script/Engine.Actor|GetRootComponent _character) (+ (Math|Vector|MakeVector 0.0 0.0 (Variables|/Script/Engine.CapsuleComponent|GetCapsuleHalfHeight (Variables|/Script/Engine.Character|GetCapsuleComponent _character))) (Transformation|GetWorldLocation (Variables|Default|GetStandLocation_exit))) (Transformation|GetActorRotation _character) false false 0.5 false)
          (Class|BPICharacter|ToggleMovement(Message) (Variables|Default|GetCharacter) true))))
    (:else)))

(event EventBeginPlay
  (|CallParentFunction) ; This node is disabled and will not be called.\nDrag off pins to build functionality.
)

(event Collision|EventActorBeginOverlap
  (params (OtherActor :type Actor%20Object%20Reference))
  (|CallParentFunction OtherActor) ; This node is disabled and will not be called.\nDrag off pins to build functionality.
)

(event EventTick
  (params (DeltaSeconds :type Float%20%28single-precision%29))
  (|CallParentFunction DeltaSeconds) ; This node is disabled and will not be called.\nDrag off pins to build functionality.
)

(event EventStartInteraction
  (params (InteractingCharacter :type Actor%20Object%20Reference))
  (|CallParentFunction InteractingCharacter)
  (bind _ascharacter (Utilities|Casting|CastToCharacter (Variables|Default|GetInteractingActor)))
  (bind _output_get (Variables|Default|SetCharacter _ascharacter))
  (Class|BPICharacter|ToggleMovement(Message) _output_get false)
  (Animation|PlayAnimMontage _output_get "/Game/Characters/Mannequins/Animations/Manny/AI_Actions/Lying_Down_Anim_Montage.Lying_Down_Anim_Montage" 1.0 "None")
  (Components|MoveComponentTo (Variables|/Script/Engine.Actor|GetRootComponent (Variables|Default|GetCharacter)) (+ (Transformation|GetActorLocation) (Math|Vector|MakeVector 0.0 0.0 (Variables|/Script/Engine.CapsuleComponent|GetCapsuleHalfHeight (Variables|/Script/Engine.Character|GetCapsuleComponent (Variables|Default|GetCharacter))))) (Math|Rotator|MakeRotator 0.0 0.0 (.yaw (Transformation|GetActorRotation))) true true 0.6 true))

(fn ConstructionScript
  (|CallParentFunction))

(fn EndInteraction
  (|CallParentFunction)
  (CallFunction|ReleaseChair)
  (return true))