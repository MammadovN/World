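; BP_Resource is an interactable pickup that grants one or more resource types to the inventory of whoever collects it.
; Its box overlap registers it with the player, and GetAction supplies the "Collect" label.
; StartInteraction runs once, disabling collision and looping through paired Type and Amounts arrays before expiring.
; The latent AddResourceM macro adds each resource, plays a sound and animates floating text before the next.
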(event OnComponentEndOverlap(Box)
  (params (OverlappedComponent :type Primitive%20Component%20Object%20Reference) (OtherActor :type Actor%20Object%20Reference) (OtherComp :type Primitive%20Component%20Object%20Reference) (OtherBodyIndex :type Integer))
  (bind _yes_no (Class|BPIChatracter|IsPlayer(Message) OtherActor))
  (if _yes_no
    (Class|BPIChatracter|RegisterInteractableActor(Message) OtherActor)))

(event OnComponentBeginOverlap(Box)
  (params (OverlappedComponent :type Primitive%20Component%20Object%20Reference) (OtherActor :type Actor%20Object%20Reference) (OtherComp :type Primitive%20Component%20Object%20Reference) (OtherBodyIndex :type Integer) (bFromSweep :type Boolean) (SweepResult :type Hit%20Result%20Structure%20%28by%20ref%29))
  (bind _yes_no (Class|BPIChatracter|IsPlayer(Message) OtherActor))
  (if _yes_no
    (Class|BPIChatracter|RegisterInteractableActor(Message) OtherActor self)))

(event EventBeginPlay)

(event Collision|EventActorBeginOverlap
  (params (OtherActor :type Actor%20Object%20Reference)))

(event EventTick
  (params (DeltaSeconds :type Float%20%28single-precision%29)))

(event EventStartInteraction
  (params (interacting_actor :type Character%20Object%20Reference))
  (bind _type (Variables|Default|Gettype))
  (bind _index (Variables|Default|Getindex))
  (bind _inventory (Class|BPIChatracter|GetInventory(Message) interacting_actor))
  (Utilities|IsValid _inventory
    (:Is%20Valid
      (Utilities|FlowControl|DoOnce false
        (:Completed
          (Collision|SetCollisionEnabled (Variables|Default|GetBox) "NoCollision")
          (if (> (Utilities|Array|Length _type) _index) :!label _label
            (Utilities|AddResourceM _inventory (Utilities|Array|Get(acopy) _type _index) (Utilities|Array|Get(acopy) (Variables|Default|Getamounts) _index)
              (:Completed
                (Math|Integer|IncrementInt (Variables|Default|Getindex)
                  (:%20%20
                    (goto _label)))))
            (else
              (Actor|SetLifeSpan 0.1))))))))

(fn ConstructionScript)

(fn GetAction
  (bind _type (Variables|Default|Gettype))
  (return (Utilities|String|Append "Collect " (select (== (Utilities|Array|Length _type) 1) (Utilities|String|EnumtoString (Utilities|Array|Get(acopy) _type)) " Resources"))))