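; BP_Arrow is an arrow actor with switchable magic types: none, fire, poison or frost.
; Next/Previous input cycles the type, highlights that inventory resource, falls back to None when out of stock, and updates attached particles and sound.
; Fire spends one resource, detaches the arrow and line traces past the target instead of simulating a projectile.
; MoveComponentTo carries it along that line, hit actors receive OnArrowHitMessage, and a short lifespan removes it.
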(event EventBeginPlay)

(event Collision|EventActorBeginOverlap
  (params (OtherActor :type Actor%20Object%20Reference)))

(event EventTick
  (params (DeltaSeconds :type Float%20%28single-precision%29)))

(event Input|ActionEvents|InputActionNextType
  (params (Key :type Key%20Structure))
  (:Pressed
    (bind _result (Math|Integer|IncrementInt (Variables|Default|Getarrow%20type%20index))
      (:%20%20
        (bind _output_get (Variables|Default|Setarrow%20type%20index (Math|Integer|Clamp(Integer) (Math|Integer|%(Integer) _result 4) 0 3)))
        (bind _inventory (Class|BPIChatracter|GetInventory(Message) (Variables|Default|Getcharacter)))
        (Variables|Default|Setresource%20type (Utilities|Select :Index _output_get :Option%200 "NewEnumerator0" :Option%201 "NewEnumerator1" :Option%202 "NewEnumerator2" :Option%203 "NewEnumerator3"))
        (bind _count (Class|BPIInventory|GetResourceCount(Message) _inventory (Utilities|Select :Index _output_get :Option%200 "NewEnumerator0" :Option%201 "NewEnumerator1" :Option%202 "NewEnumerator2" :Option%203 "NewEnumerator3")))
        (Class|BPIInventory|HighLightResource(Message) _inventory (Utilities|Select :Index _output_get :Option%200 "NewEnumerator0" :Option%201 "NewEnumerator1" :Option%202 "NewEnumerator2" :Option%203 "NewEnumerator3"))
        (Development|PrintString (Utilities|String|ToString(Integer) _count))
        (Variables|Default|SetMagicType (Utilities|Select :Index (Math|Integer|SelectInt _output_get 0 (> _count 0)) :Option%200 "NewEnumerator0" :Option%201 "NewEnumerator1" :Option%202 "NewEnumerator2" :Option%203 "NewEnumerator3"))
        (Development|PrintString (Utilities|String|ToString(Integer) (Variables|Default|Getarrow%20type%20index)))
        (Utilities|IsValid (Variables|Default|Getarrow%20particle)
          (:Is%20Valid
            (Components|DestroyComponent (Variables|Default|Getarrow%20particle)))
          (:Is%20Not%20Valid
            _))
        (Audio|Components|Audio|Stop (Variables|Default|Getarrow%20fire%20sound))
        (Utilities|IsValid (Utilities|Select :Index (Variables|Default|GetMagicType) :NewEnumerator0 0 :NewEnumerator1 "/Game/StarterContentMin/Particles/P_Fire1.P_Fire1" :NewEnumerator2 "/Game/StarterContentMin/Particles/P_FireGreen.P_FireGreen" :NewEnumerator3 "/Game/StarterContentMin/Particles/P_FireBlue.P_FireBlue")
          (:Is%20Valid
            (bind _returnvalue (Effects|SpawnEmitterAttached (Utilities|Select :Index (Variables|Default|GetMagicType) :NewEnumerator0 0 :NewEnumerator1 "/Game/StarterContentMin/Particles/P_Fire1.P_Fire1" :NewEnumerator2 "/Game/StarterContentMin/Particles/P_FireGreen.P_FireGreen" :NewEnumerator3 "/Game/StarterContentMin/Particles/P_FireBlue.P_FireBlue") (Variables|Default|Getparticle%20socket) "None" "0, 0, 0" "0, 0, 0" "0.200000,0.200000,0.200000"))
            (Variables|Default|Setarrow%20particle _returnvalue)
            (Audio|Components|Audio|Play (Variables|Default|Getarrow%20fire%20sound) 0.0)))))))

(event Input|ActionEvents|InputActionPreviousType
  (params (Key :type Key%20Structure))
  (:Pressed
    (Math|Integer|DecrementInt (Variables|Default|Getarrow%20type%20index)
      (:%20%20
        (bind _output_get (Variables|Default|Setarrow%20type%20index (Math|Integer|Clamp(Integer) (Math|Integer|%(Integer) (stale Input|ActionEvents|InputActionNextType _result) 4) 0 3)))
        (bind _inventory (Class|BPIChatracter|GetInventory(Message) (Variables|Default|Getcharacter)))
        (Variables|Default|Setresource%20type (Utilities|Select :Index _output_get :Option%200 "NewEnumerator0" :Option%201 "NewEnumerator1" :Option%202 "NewEnumerator2" :Option%203 "NewEnumerator3"))
        (bind _count (Class|BPIInventory|GetResourceCount(Message) _inventory (Utilities|Select :Index _output_get :Option%200 "NewEnumerator0" :Option%201 "NewEnumerator1" :Option%202 "NewEnumerator2" :Option%203 "NewEnumerator3")))
        (Class|BPIInventory|HighLightResource(Message) _inventory (Utilities|Select :Index _output_get :Option%200 "NewEnumerator0" :Option%201 "NewEnumerator1" :Option%202 "NewEnumerator2" :Option%203 "NewEnumerator3"))
        (Development|PrintString (Utilities|String|ToString(Integer) _count))
        (Variables|Default|SetMagicType (Utilities|Select :Index (Math|Integer|SelectInt _output_get 0 (> _count 0)) :Option%200 "NewEnumerator0" :Option%201 "NewEnumerator1" :Option%202 "NewEnumerator2" :Option%203 "NewEnumerator3"))
        (Development|PrintString (Utilities|String|ToString(Integer) (Variables|Default|Getarrow%20type%20index)))
        (Utilities|IsValid (Variables|Default|Getarrow%20particle)
          (:Is%20Valid
            (Components|DestroyComponent (Variables|Default|Getarrow%20particle)))
          (:Is%20Not%20Valid
            _))
        (Audio|Components|Audio|Stop (Variables|Default|Getarrow%20fire%20sound))
        (Utilities|IsValid (Utilities|Select :Index (Variables|Default|GetMagicType) :NewEnumerator0 0 :NewEnumerator1 "/Game/StarterContentMin/Particles/P_Fire1.P_Fire1" :NewEnumerator2 "/Game/StarterContentMin/Particles/P_FireGreen.P_FireGreen" :NewEnumerator3 "/Game/StarterContentMin/Particles/P_FireBlue.P_FireBlue")
          (:Is%20Valid
            (bind _returnvalue (Effects|SpawnEmitterAttached (Utilities|Select :Index (Variables|Default|GetMagicType) :NewEnumerator0 0 :NewEnumerator1 "/Game/StarterContentMin/Particles/P_Fire1.P_Fire1" :NewEnumerator2 "/Game/StarterContentMin/Particles/P_FireGreen.P_FireGreen" :NewEnumerator3 "/Game/StarterContentMin/Particles/P_FireBlue.P_FireBlue") (Variables|Default|Getparticle%20socket) "None" "0, 0, 0" "0, 0, 0" "0.200000,0.200000,0.200000"))
            (Variables|Default|Setarrow%20particle _returnvalue)
            (Audio|Components|Audio|Play (Variables|Default|Getarrow%20fire%20sound) 0.0)))))))

(fn ConstructionScript)

(event Custom|Fire
  (params (target :type Vector) (source%20actor :type Actor%20Object%20Reference))
  (bind _self self)
  (bind _defaultsceneroot (Variables|Default|GetDefaultSceneRoot))
  (bind _returnvalue (Transformation|GetActorLocation _self))
  (bind _returnvalue_2 (Math|Rotator|FindLookatRotation _returnvalue target))
  (bind _returnvalue_3 (Math|Vector|GetUnitDirection(Vector) _returnvalue target))
  (bind _inventory (Class|BPIChatracter|GetInventory(Message) (Variables|Default|Getcharacter)))
  (Class|BPIInventory|UpdateResourceCount(Message) _inventory (Variables|Default|Getresource%20type) -1)
  (Development|PrintString "arrow shot" true true "(R=0.000000,G=0.660000,B=1.000000,A=1.000000)" 2e+02)
  (Audio|Components|Audio|Play (Variables|Default|GetSK_Trail) true)
  (Transformation|SetWorldRotation (Variables|Default|GetDefaultSceneRoot) _returnvalue_2 false false)
  (Audio|PlaySoundatLocation "/Game/Audio/Weapon/SC_Swoosh.SC_Swoosh" _returnvalue "0, 0, 0" 1.0 1.0 0.0 0 0 0)
  (Transformation|DetachFromComponent _defaultsceneroot "KeepWorld" "KeepWorld" "KeepWorld" true)
  (bind (_outhit _returnvalue_4) (Collision|LineTraceByChannel _returnvalue (+ target (* _returnvalue_3 5e+02)) "TraceTypeQuery1" false (Utilities|Array|MakeArray source%20actor) "None"))
  (if _returnvalue_4
    (Components|MoveComponentTo (Variables|Default|GetDefaultSceneRoot) (.location _outhit) _returnvalue_2 false false 0.2 false)
    (Transformation|SetRelativeLocation (Variables|Default|Getarrow) "-30.000000, 0, 0" false false)
    (Class|BPIDamageable|OnArrowHit(Message) (.hitactor _outhit) (.location _outhit) source%20actor self)
    (Audio|Components|Audio|Stop (Variables|Default|GetSK_Trail))
    (Development|PrintString (Utilities|String|Append "hit on - " (Utilities|GetDisplayName (.hitactor _outhit))) true true "(R=0.000000,G=0.660000,B=1.000000,A=1.000000)" 2e+02)
    (Actor|SetLifeSpan 1.0)
    (else
      (Components|MoveComponentTo _defaultsceneroot (+ target (* _returnvalue_3 5e+03)) _returnvalue_2 false false 0.2 false)
      (Development|PrintString "no hit" true true "(R=0.000000,G=0.660000,B=1.000000,A=1.000000)" 2e+02)
      (Actor|SetLifeSpan 0.01))))

(fn GetMagicType
  (return (Variables|Default|GetMagicType)))