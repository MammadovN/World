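; BP_Bow is a bow weapon Blueprint that drives the animations of its Bow skeletal mesh.
; Toggling charge plays a non-looping montage asset when enabled and the base bow animation when disabled.
; Firing plays the Bow_Fire montage on the mesh at a greatly increased play rate.
; The custom depth toggle calls the parent implementation, then applies the setting to the Bow mesh.
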(event EventBeginPlay
  (|CallParentFunction) ; This node is disabled and will not be called.\nDrag off pins to build functionality.
)

(event Collision|EventActorBeginOverlap
  (params (OtherActor :type Actor%20Object%20Reference))
  (|CallParentFunction OtherActor) ; This node is disabled and will not be called.\nDrag off pins to build functionality.
)

(event EventTick
  (params (DeltaSeconds :type Float%20%28single-precision%29))
  (|CallParentFunction DeltaSeconds) ; This node is disabled and will not be called.\nDrag off pins to build functionality.
)

(event EventToggleChargeWeapon
  (params (enable :type Boolean))
  (bind _bow (Variables|Default|GetBow))
  (if enable
    (Components|Animation|PlayAnimation _bow "/Game/BP/Weapons/Bow_and_Arrow/Bow_Anim_Montage.Bow_Anim_Montage" false)
    (else
      (Components|Animation|PlayAnimation _bow "/Game/BP/Weapons/Bow_and_Arrow/Bow_Anim.Bow_Anim" false))))

(event EventFire
  (Animation|Montage|PlayMontage (Variables|Default|GetBow) "/Game/BP/Weapons/Bow_and_Arrow/Bow_Fire.Bow_Fire" 1e+01))

(event EventToggleCustomDepth
  (params (enable :type Boolean))
  (|CallParentFunction enable)
  (Rendering|SetRenderCustomDepth (Variables|Default|GetBow) enable))

(fn ConstructionScript
  (|CallParentFunction))