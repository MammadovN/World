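; BP_Inventory is a quiver actor that tracks its parent actor's resource counts, including arrows.
; AddtoInventory updates the ResourceCounts map, then pushes count changes to the HUD if the parent is the player, as do highlight requests.
; Arrow functions check, report and decrement the count, or spawn a BP_Arrow owned by the parent character; ConsumeArrow skips the HUD update.
; ToggleCustomDepth switches custom depth rendering on the quiver and arrow meshes.
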(event EventBeginPlay)

(event Collision|EventActorBeginOverlap
  (params (OtherActor :type Actor%20Object%20Reference)))

(event EventTick
  (params (DeltaSeconds :type Float%20%28single-precision%29)))

(event EventAddtoInventory
  (params (resource%20type :type ResourceTypes%20Enum :default "NewEnumerator0") (amount :type Integer))
  (CallFunction|UpdateResourceCount resource%20type amount))

(event EventHighLightResource
  (params (resource%20type%20 :type ResourceTypes%20Enum :default "NewEnumerator0"))
  (bind _yes_no (Class|BPIChatracter|IsPlayer(Message) (Actor|GetParentActor)))
  (if _yes_no
    (Class|BPIUI|HighLightResource(Message) (HUD|GetHUD (Game|GetPlayerController 0)) resource%20type%20)))

(event EventUpdateResourceCount
  (params (resource%20index :type ResourceTypes%20Enum :default "NewEnumerator0") (change :type Integer))
  (bind _resource_counts (Variables|Default|Getresource%20counts))
  (bind _value (Utilities|Map|Find _resource_counts resource%20index))
  (Utilities|Map|Add _resource_counts resource%20index (+ _value change))
  (bind _yes_no (Class|BPIChatracter|IsPlayer(Message) (Actor|GetParentActor)))
  (if _yes_no
    (Class|BPIUI|UpdateResourceCount(Message) (HUD|GetHUD (Game|GetPlayerController 0)) resource%20index _value)))

(event EventToggleCustomDepth
  (params (enable :type Boolean))
  (Rendering|SetRenderCustomDepth (Variables|Default|GetQuiver) enable))

(fn ConstructionScript)

(fn HasArrows?
  (bind _resource_counts (Variables|Default|Getresource%20counts))
  (bind (_value _returnvalue) (Utilities|Map|Find _resource_counts "NewEnumerator4"))
  (if _returnvalue
    (return (> _value 0))
    (else
      (return false))))

(fn GetArrow
  (bind _returnvalue (Game|SpawnActorfromClass "/Game/BP/Weapons/BP_Arrow.BP_Arrow_C" (Math|Transform|MakeTransform "0, 0, 0" "0, 0, 0" "1,1,1") "AlwaysSpawn" 0 0))
  (Variables|/Game/BP/Weapons/BP_Arrow.BP_Arrow_C|Setcharacter _returnvalue (Actor|GetParentActor))
  (return _returnvalue))

(fn GetArrowCount
  (return (.Value (Utilities|Map|Find (Variables|Default|Getresource%20counts) "NewEnumerator4")) (Variables|Default|Getcapacity)))

(fn ConsumeArrow
  (bind _resource_counts (Variables|Default|Getresource%20counts))
  (bind _value (Utilities|Map|Find _resource_counts "NewEnumerator4"))
  (Utilities|Map|Add _resource_counts "NewEnumerator4" (Math|Integer|Clamp(Integer) (- _value 1) 0 _value)))

(fn GetResourceCount
  (params (resource%20index :type ResourceTypes%20Enum :default "NewEnumerator0"))
  (return (.Value (Utilities|Map|Find (Variables|Default|Getresource%20counts) resource%20index))))